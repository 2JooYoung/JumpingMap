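; Behavior Tree service that lets an AI pawn detect the player by proximity.
; On activation it waits briefly, then finds and caches the BP_Player actor.
; Each tick, if that reference is valid, it writes the player to the Player blackboard key when within a fixed radius of the controlled pawn, otherwise clears the key.
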(event EventReceiveTickAI
  (params (OwnerController :type AI%20Controller%20Object%20Reference) (ControlledPawn :type Pawn%20Object%20Reference) (DeltaSeconds :type Float%20%28single-precision%29))
  (bind _bpplayer (Variables|Default|GetBPPlayer))
  (Utilities|IsValid _bpplayer
    (:Is%20Valid
      (if (< (Math|Vector|VectorLength (- (Transformation|GetActorLocation _bpplayer) (Transformation|GetActorLocation ControlledPawn))) 1e+03)
        (Class|BTFunctionLibrary|SetBlackboardValueasObject (Variables|Default|GetPlayer) (Variables|Default|GetBPPlayer))
        (else
          (Class|BTFunctionLibrary|SetBlackboardValueasObject (Variables|Default|GetPlayer)))))))

(event EventReceiveActivationAI
  (params (OwnerController :type AI%20Controller%20Object%20Reference) (ControlledPawn :type Pawn%20Object%20Reference))
  ;[0.15 0.15 0.15 0.5] 딱한번 실행
  (Utilities|FlowControl|Delay 1.0)
  (bind _returnvalue (Actor|GetActorOfClass "/Game/BluePrints/BP_Player.BP_Player_C"))
  (Variables|Default|SetBPPlayer _returnvalue))
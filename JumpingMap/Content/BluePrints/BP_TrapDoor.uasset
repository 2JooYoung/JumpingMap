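; BP_TrapDoor is a trap door actor that swings open and closed when the player controller signals it.
; On BeginPlay it binds its open and close events to the first BP_PlayerController.
; Each event drives its own timeline, played forward to open and reversed to close, lerping the Pivot component's relative pitch through a quarter turn.
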(event Custom|CloseTrapDoor
  (bind _beta (Timeline|Timeline_0 ReverseFromEnd)
    (:Update
      (Transformation|SetRelativeRotation (Variables|Default|GetPivot) (Math|Rotator|MakeRotator 0.0 (Math|Float|Lerp 0.0 -9e+01 _beta) 0.0) false false))))

(event Custom|OpenTrapDoor
  (bind _beta (Timeline|Timeline PlayFromStart)
    (:Update
      (Transformation|SetRelativeRotation (Variables|Default|GetPivot) (Math|Rotator|MakeRotator 0.0 (Math|Float|Lerp 0.0 -9e+01 _beta) 0.0) false false))))

(event EventBeginPlay
  (bind _asbp_player_controller (Utilities|Casting|CastToBP_PlayerController (Game|GetPlayerController 0)))
  (Utilities|IsValid _asbp_player_controller
    (:Is%20Valid
      (bind _output_get (Variables|Default|SetPlayerController _asbp_player_controller))
      (EventDispatchers|BindEventtoOpen _output_get (delegate Custom|OpenTrapDoor))
      (EventDispatchers|BindEventtoClose _output_get (delegate Custom|CloseTrapDoor)))))

(fn ConstructionScript)
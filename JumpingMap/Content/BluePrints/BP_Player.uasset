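; Player Blueprint with a Fire function that shoots balloons at the screen center, plus debug prints for capsule hit and overlap events.
; Fire plays a montage, traces from the deprojected screen center, then traces from FireSocket to that hit location.
; A BP_Balloon hit by the second trace gets Boom called, and both traces draw debug lines.
; Ammo counting and other trace experiments are left unconnected.
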(event OnComponentHit(CapsuleComponent)
  (params (HitComponent :type Primitive%20Component%20Object%20Reference) (OtherActor :type Actor%20Object%20Reference) (OtherComp :type Primitive%20Component%20Object%20Reference) (NormalImpulse :type Vector :default "0, 0, 0") (Hit :type Hit%20Result%20Structure%20%28by%20ref%29))
  (Development|PrintString "Player Hit"))

(event OnComponentBeginOverlap(CapsuleComponent)
  (params (OverlappedComponent :type Primitive%20Component%20Object%20Reference) (OtherActor :type Actor%20Object%20Reference) (OtherComp :type Primitive%20Component%20Object%20Reference) (OtherBodyIndex :type Integer) (bFromSweep :type Boolean) (SweepResult :type Hit%20Result%20Structure%20%28by%20ref%29))
  (Development|PrintString "Player Begin"))

(event OnComponentEndOverlap(CapsuleComponent)
  (params (OverlappedComponent :type Primitive%20Component%20Object%20Reference) (OtherActor :type Actor%20Object%20Reference) (OtherComp :type Primitive%20Component%20Object%20Reference) (OtherBodyIndex :type Integer))
  (Development|PrintString "Player End"))

(fn ConstructionScript)

(fn Fire
  (bind _returnvalue (Viewport|GetViewportSize))
  (bind _returnvalue_2 (Game|GetPlayerController 0))
  (bind _returnvalue_3 (/ (.x _returnvalue) 2.0))
  (bind _returnvalue_4 (/ (.y _returnvalue) 2.0))
  (bind (_worldposition _worlddirection) (Class|GameplayStatics|DeprojectScreentoWorld _returnvalue_2 (Math|Vector2D|MakeVector2D _returnvalue_3 _returnvalue_4)))
  (Animation|PlayAnimMontage "/Game/Animations/AM_Fire.AM_Fire" 1.0 "Fire")
  (bind _outhit (Collision|LineTraceByChannel _worldposition (+ _worldposition (* _worlddirection 5e+03)) "TraceTypeQuery1" false 0 "ForDuration"))
  (bind _outhit_2 (Collision|LineTraceByChannel (.location (Transformation|GetSocketTransform (Variables|Character|GetMesh) "FireSocket" "RTS_World")) (.Location (Collision|BreakHitResult _outhit)) "TraceTypeQuery1" false 0 "ForDuration" true "(R=1.000000,G=0.000000,B=0.583761,A=1.000000)" "(R=0.000000,G=0.011430,B=1.000000,A=1.000000)"))
  (bind _asbp_balloon (Utilities|Casting|CastToBP_Balloon (.HitActor (Collision|BreakHitResult _outhit_2))))
  (Default|Boom _asbp_balloon))
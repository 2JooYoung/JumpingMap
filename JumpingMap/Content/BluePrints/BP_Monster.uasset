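; BP_Monster is an enemy that chases the player at close range and wanders otherwise.
; Each Tick it measures the vector to player 0's pawn and, within a fixed radius, moves along it and rotates to face it.
; Outside that radius it feeds movement input toward a random world-space point re-rolled every frame, without updating rotation.
; Movement uses direct input, with no navigation or pathfinding.
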(event EventTick
  (params (DeltaSeconds :type Float%20%28single-precision%29))
  (bind _returnvalue (Math|Random|RandomInteger 5000))
  (Variables|Default|SetDistance (- (Transformation|GetActorLocation (Game|Player|GetPlayerPawn 0)) (Transformation|GetActorLocation)))
  (if (<= (Math|Vector|VectorLength (Variables|Default|GetDistance)) 5e+02)
    (Pawn|Input|AddMovementInput (Variables|Default|GetDistance) 1.0 false)
    (Transformation|SetActorRotation (Math|Conversions|RotationFromXVector (Variables|Default|GetDistance)))
    (else
      (Variables|Default|SetRandomLocation (Math|Vector|MakeVector (Math|Conversions|ToFloat(Integer) _returnvalue) (Math|Conversions|ToFloat(Integer) _returnvalue) 0.0))
      (Pawn|Input|AddMovementInput (- (Variables|Default|GetRandomLocation) (Transformation|GetActorLocation)) 1.0 false))))

(fn ConstructionScript)
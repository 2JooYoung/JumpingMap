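; BP_TrapBall is a trap ball whose mesh moves vertically in response to the player controller's open and close events.
; On BeginPlay it casts player 0's controller to BP_PlayerController and binds LaunchBall to open and ReverseBall to close.
; LaunchBall plays one timeline and ReverseBall reverses a separate one, each lerping the static mesh's relative Z location over the same range.
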(event Custom|LaunchBall
  (bind _alpha (Timeline|Timeline Play)
    (:Update
      (Transformation|SetRelativeLocation (Variables|Default|GetStaticMesh) (Math|Vector|MakeVector 0.0 0.0 (Math|Float|Lerp 0.0 1e+02 _alpha)) false false))))

(event Custom|ReverseBall
  (bind _alpha (Timeline|Timeline_0 Reverse)
    (:Update
      (Transformation|SetRelativeLocation (Variables|Default|GetStaticMesh) (Math|Vector|MakeVector 0.0 0.0 (Math|Float|Lerp 0.0 1e+02 _alpha)) false false))))

(event EventBeginPlay
  (bind _asbp_player_controller (Utilities|Casting|CastToBP_PlayerController (Game|GetPlayerController 0)))
  (Utilities|IsValid _asbp_player_controller
    (:Is%20Valid
      (bind _output_get (Variables|Default|SetPlayerController _asbp_player_controller))
      (EventDispatchers|BindEventtoOpen _output_get (delegate Custom|LaunchBall))
      (EventDispatchers|BindEventtoClose _output_get (delegate Custom|ReverseBall)))))

(fn ConstructionScript)
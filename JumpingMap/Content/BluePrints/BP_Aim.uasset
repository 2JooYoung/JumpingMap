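; BP_Aim is a HUD Blueprint that shows an aiming crosshair at the center of the screen.
; Every frame, DrawHUD draws the CrossHair texture at a fixed size, offset by half that size from the viewport midpoint to keep it centered.
; On BeginPlay it also creates a WBP_TestWidget, stores the reference and adds it to the viewport.
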(event EventBeginPlay
  (bind _returnvalue (UserInterface|CreateWidget "/Game/Test/WBP_TestWidget.WBP_TestWidget_C"))
  (bind _output_get (Variables|Default|SetTestWidget _returnvalue))
  (UserInterface|Viewport|AddtoViewport _output_get 0))

(event EventDrawHUD
  (params (SizeX :type Integer) (SizeY :type Integer))
  ;[0.15 0.15 0.15 0.5] 화면 크기 전달
  ; 매 프레임마다 호출.
  ; 매 플레임마다 화면 그림
  (Canvas|DrawTexture "/Game/Assets/CrossHair.CrossHair" (Math|Conversions|ToFloat(Integer) (- (/ SizeX 2) 24)) (Math|Conversions|ToFloat(Integer) (- (/ SizeY 2) 24)) 48.0 48.0 0.0 0.0 1.0 1.0 "(R=1.000000,G=1.000000,B=1.000000,A=1.000000)"))

(fn ConstructionScript)